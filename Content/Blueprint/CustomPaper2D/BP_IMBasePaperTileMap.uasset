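; BP_IMBasePaperTileMap is a Paper2D tile map actor that randomly changes its colored background.
; Tick accumulates delta time and, every two seconds, sets the RenderComponent's tile map to one of six background color variants chosen at random.
; The same variant can repeat, since the pick ignores the current one.
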(event `self.ReceiveTick`
  (params (DeltaSeconds :type "Float (single-precision)"))
  (set `self.NowTime` (+ DeltaSeconds (`self.NowTime`)))
  (if (> (`self.NowTime`) 2.0)
    (set `self.NowTime` (- (`self.NowTime`) 2.0))
    (`PaperTileMapComponent.SetTileMap` (`self.RenderComponent`) (select `int` (`KismetMathLibrary.RandomInteger` 6) :`0` "/Game/TileMaps/TM_Background_Blue.TM_Background_Blue" :`1` "/Game/TileMaps/TM_Background_Brown.TM_Background_Brown" :`2` "/Game/TileMaps/TM_Background_Gray.TM_Background_Gray" :`3` "/Game/TileMaps/TM_Background_Green.TM_Background_Green" :`4` "/Game/TileMaps/TM_Background_Pink.TM_Background_Pink" :`5` "/Game/TileMaps/TM_Background_Purple.TM_Background_Purple" :!type "PaperTileMap Object Reference"))))

(fn `UserConstructionScript`)